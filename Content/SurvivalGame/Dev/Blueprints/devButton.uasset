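; Dev interactable button that switches a light, identified by its LightID, on or off through a referenced lighting controller.
; On interaction with its sphere, it flips IsOn and passes the state to the controller, provided the controller allows a light change.
; A dynamic material instance on the sphere shows the state with teal emissive for on and red for off.
; Interaction is refused while the button is disabled.
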(event `self.ReceiveBeginPlay`
  (bind _returnvalue (`PrimitiveComponent.CreateDynamicMaterialInstance` (`self.Sphere`) 0 "/Game/SurvivalGame/Dev/Blueprints/ButtonMaterial.ButtonMaterial" "None"))
  (set `self.ButtonMaterial` _returnvalue)
  (`self.UpdateGraphics`))

(event `UpdateGraphics`
  (`MaterialInstanceDynamic.SetVectorParameterValue` (`self.ButtonMaterial`) "Emissive" (select `bool` (`self.IsOn`) :`false` (struct :`R` 0.5 :`A` 1.0) :`true` (struct :`G` 0.5 :`B` 0.5 :`A` 1.0) :!type "LinearColor Structure")))

(event `InteractionInterface.BeginInteraction`
  (params (Info :type "InteractionInfo Structure"))
  (if (`/Game/SurvivalGame/Dev/Blueprints/LightingController.CanChangeLight` (`self.LightingControllerRef`))
    (if (== (`.HitComponent` (break `InteractionInfo` Info)) (`self.Sphere`))
      (set `self.IsOn` (not (`self.IsOn`)))
      (`self.UpdateGraphics`)
      (`/Game/SurvivalGame/Dev/Blueprints/LightingController.SetLightEnabled` (`self.LightingControllerRef`) (`self.IsOn`) (`self.LightID`)))))

(fn `CanInteract`
  (params (Info :type "InteractionInfo Structure"))
  (returns (ReturnValue :type Boolean))
  (return (not (`self.IsDisabled`))))

(fn `UserConstructionScript`)