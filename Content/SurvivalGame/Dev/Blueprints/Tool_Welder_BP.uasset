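; Welder tool Blueprint that adds particle effects on top of its parent tool's primary and secondary actions.
; Both actions call the parent, then activate the welder particle system.
; When the last hit distance is within tool range, sparks activate slightly off the impact point toward the trace start, or at the emitter location without a blocking hit.
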(event `self.OnPrimaryAction`
  (bind (_bblockinghit _binitialoverlap _time _distance _location _impactpoint _normal _impactnormal _physmat _hitactor _hitcomponent _hitbonename _hititem _faceindex _tracestart) (`GameplayStatics.BreakHitResult` (`self.LastHitResult`)))
  (`parent.OnPrimaryAction`)
  (`ActorComponent.Activate` (`self.Welder_PS`) true :!label _label)
  (if (> (`self.ToolRange`) _distance)
    (`SceneComponent.K2_SetWorldLocation` (`self.Sparks_PS`) (select `bool` _bblockinghit :`false` (`SceneComponent.K2_GetComponentLocation` (`self.ParticleEmitterLocation`)) :`true` (+ _impactpoint (* (`KismetMathLibrary.GetDirectionUnitVector` _impactpoint _tracestart) 20.0))) false false)
    (`ActorComponent.Activate` (`self.Sparks_PS`) true)))

(event `self.OnSecondaryAction`
  (`parent.OnSecondaryAction`)
  (goto _label))

(fn `UserConstructionScript`)