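; DevShelfChest is a shelf storage container whose visible item meshes reflect how full its inventory is.
; The construction script builds an ordered array of filler meshes, which BeginPlay gives small random yaw and position offsets for a less uniform look.
; On BeginPlay and whenever an InventoryManager slot changes, it shows a rounded share of those meshes proportional to the occupied slots and hides the rest.
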(event `self.ReceiveBeginPlay`
  (add `InventoryManager.OnInventoryManagerSlotChangedDispatcher` (`self.InventoryManager`) (delegate `UpdateGraphics`))
  (`self.UpdateGraphics` 0)
  (for _array_element (`self.ShelfFillerMeshes`)
    (`SceneComponent.K2_SetRelativeRotation` _array_element (`KismetMathLibrary.MakeRotator` 0.0 0.0 (`KismetMathLibrary.RandomFloatInRange` -10.0 10.0)) false false)
    (`SceneComponent.K2_AddLocalOffset` _array_element (`KismetMathLibrary.MakeVector` (* (.x (`KismetMathLibrary.RandomUnitVector`)) 5.0) (* (.y (`KismetMathLibrary.RandomUnitVector`)) 10.0)) false false)))

(event `UpdateGraphics`
  (params (TargetSlot :type Integer))
  (bind _inventorymanager (`self.InventoryManager`))
  (for (_array_element _array_index) (`self.ShelfFillerMeshes`)
    (`SceneComponent.SetVisibility` _array_element (< _array_index (`KismetMathLibrary.Round` (* (`KismetArrayLibrary.Array_Length` (`self.ShelfFillerMeshes`)) (- 1.0 (/ (`KismetMathLibrary.Conv_IntToDouble` (`KismetArrayLibrary.Array_Length` (`InventoryManager.FindEmptySlots` _inventorymanager))) (`KismetMathLibrary.Conv_IntToDouble` (`InventoryManager.GetInventorySize` _inventorymanager))))))) false)))

(fn `UserConstructionScript`
  (set `self.ShelfFillerMeshes` (`|MakeArray` (`self.SM_GenericItem6`) (`self.SM_GenericItem7`) (`self.SM_GenericItem8`) (`self.SM_GenericItem9`) (`self.SM_GenericItem10`) (`self.SM_GenericItem11`) (`self.SM_GenericItem3`) (`self.SM_GenericItem4`) (`self.SM_GenericItem5`) (`self.SM_GenericItem13`) (`self.SM_GenericItem14`) (`self.SM_GenericItem12`))))