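; Player character Blueprint for the survival game, which passes its team ID to the team player controller on BeginPlay.
; Crouch events call the parent logic and shift the camera attachment down or up to match.
; The inventory event toggles the menu: it closes an open widget or creates one fed by the hotbar and inventory managers.
; Construction caches capsule half-height and attaches hotbar tools to the hands mesh's grip socket.
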(event `self.ReceiveBeginPlay`
  (bind _asteam_player_controller (cast `TeamPlayerController` (`self.GetController`)))
  (`TeamPlayerController.SetTeamID` _asteam_player_controller (`self.TeamID`)))

(event `self.StartCrouch`
  (`parent.StartCrouch`))

(event `self.StopCrouching`
  (`parent.StopCrouching`))

(event `self.K2_OnStartCrouch`
  (params (HalfHeightAdjust :type "Float (single-precision)") (ScaledHalfHeightAdjust :type "Float (single-precision)"))
  (`parent.K2_OnStartCrouch` HalfHeightAdjust ScaledHalfHeightAdjust)
  (`SceneComponent.K2_AddRelativeLocation` (`self.CameraAttachmentComponent`) (0.0 0.0 -40.0) false false))

(event `self.K2_OnEndCrouch`
  (params (HalfHeightAdjust :type "Float (single-precision)") (ScaledHalfHeightAdjust :type "Float (single-precision)"))
  (`parent.K2_OnEndCrouch` HalfHeightAdjust ScaledHalfHeightAdjust)
  (`SceneComponent.K2_AddRelativeLocation` (`self.CameraAttachmentComponent`) (0.0 0.0 40.0) false false))

(event `self.OnOpenInventory`
  (`/Engine/EditorBlueprintResources/StandardMacros.IsValid` (`self.InventoryHUDWidget`)
    (:`Is Valid`
      (`/Engine/EditorBlueprintResources/StandardMacros.IsValid` (`Widget.GetParent` (`self.InventoryHUDWidget`))
        (:`Is Valid`
          (message `MenuInterface.CloseMenu` (`self.InventoryHUDWidget`)))
        (:`Is Not Valid`
          (`Widget.RemoveFromParent` (`self.InventoryHUDWidget`))
          (`self.SetInventoryHUDWidget` null)
          (bind _asplayer_controller (cast `PlayerController` (`self.GetController`) :!label _label))
          (bind _returnvalue (`|CreateWidget` "/Game/SurvivalGame/Dev/UI/HUD_InventoryMenu.HUD_InventoryMenu_C" _asplayer_controller (`self.HotbarManagerRef`) (`self.InventoryManagerRef`)))
          (`self.SetInventoryHUDWidget` _returnvalue)
          (`UserWidget.AddToViewport` (`self.InventoryHUDWidget`) 0)
          (message `MenuInterface.OpenMenu` (`self.InventoryHUDWidget`)))))
    (:`Is Not Valid`
      (goto _label))))

(event `self.ReceiveTick`
  (params (DeltaSeconds :type "Float (single-precision)"))
  (`parent.ReceiveTick` DeltaSeconds))

(fn `UserConstructionScript`
  (set `self.DefaultCapsuleHalfHeight` (`CapsuleComponent.CapsuleHalfHeight` (`self.CapsuleComponent`)))
  (`HotbarManager.SetToolAttachment` (`self.HotbarManagerRef`) (`self.HandsMesh`) "GripPoint"))