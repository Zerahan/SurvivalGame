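; DevChest is a development chest Blueprint whose lid swings open when a player interacts with it.
; It extends its parent's begin and cancel interaction events, then checks the interacting controller reference.
; A valid reference on begin plays a lid timeline that pitches the Hinge component by its scaled Rotation track.
; Cancelling reverses the timeline to close the lid only when no valid controller reference remains.
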(event `InteractionInterface.BeginInteraction`
  (params (Info :type "InteractionInfo Structure"))
  (`parent.BeginInteraction` Info)
  (`/Engine/EditorBlueprintResources/StandardMacros.IsValid` (`self.InteractingControllerRef`)
    (:`Is Valid`
      (bind (_direction _rotation) (`Timeline|LidTimeline` :!label _label)
        (:`Update`
          (`SceneComponent.K2_SetRelativeRotation` (`self.Hinge`) (`KismetMathLibrary.MakeRotator` 0.0 (* _rotation 50.0)) false false))))))

(event `InteractionInterface.CancelInteraction`
  (params (Info :type "InteractionInfo Structure"))
  (`parent.CancelInteraction` Info)
  (`/Engine/EditorBlueprintResources/StandardMacros.IsValid` (`self.InteractingControllerRef`)
    (:`Is Not Valid`
      (goto _label :!via `Reverse`))))

(fn `UserConstructionScript`)