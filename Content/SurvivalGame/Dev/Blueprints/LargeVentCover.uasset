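; Large vent cover door that can be opened, closed, broken and repaired, extending a parent door class through its open, close, break and repair events.
; A timeline slides and rotates the cover toward an open transform and sets the door state when finished.
; Breaking or repairing swaps the mesh, toggles collision on the cover and vision blocker, and updates health state.
; Construction and BeginPlay both apply the saved door and health states.
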(event `self.ReceiveBeginPlay`
  (`|ExecutionSequence`
    (:`then_0`
      (switch `EDoorState` (`self.CurrentDoorState`)
        (:`IsClosed`
          (`self.SetDoorPosition` false))
        (:`IsOpen`
          (`self.SetDoorPosition` true))))
    (:`then_1`
      (switch `EHealthState` (`self.StatusHealthState`)
        (:`IsAlive`
          (`self.SetRepaired`))
        (:`IsDead`
          (`self.SetBroken`))))))

(event `self.OnOpen`
  (`parent.OnOpen`)
  (bind (_direction _doorlocationa _doorlocationb) (`Timeline|VentCoverTimeline` :`NewTime` (select `bool` (stale `SetDoorPosition` IsOpen) :`true` 0.5 :!type "Float (single-precision)") :!label _label)
    (:`Update`
      (`SceneComponent.K2_SetRelativeLocationAndRotation` (`self.VentCover`) (.location (`KismetMathLibrary.TLerp` (`KismetMathLibrary.MakeTransform` (`KismetMathLibrary.MakeVector` (* _doorlocationa 10.0))) (`self.DoorOpenTransform`) _doorlocationb)) (.rotation (`KismetMathLibrary.TLerp` (`KismetMathLibrary.MakeTransform` (`KismetMathLibrary.MakeVector` (* _doorlocationa 10.0))) (`self.DoorOpenTransform`) _doorlocationb)) false false))
    (:`Finished`
      (`self.SetDoorState` (select `bool` (`|EnumEquality` _direction "Forward") :`false` "IsClosed" :`true` "IsOpen" :!type "EDoorState Enum")))))

(event `self.OnClose`
  (`parent.OnClose`)
  (goto _label :!via `Reverse`))

(event `SetDoorPosition`
  (params (IsOpen :type Boolean))
  (goto _label :!via `SetNewTime`))

(event `self.OnBreakDoor`
  (`parent.OnBreakDoor`)
  (`StaticMeshComponent.SetStaticMesh` (`self.VentCover`) "/Game/SurvivalGame/Dev/Meshes/DetatchableVentCover_Large_VentCover_Destroyed_MESH.DetatchableVentCover_Large_VentCover_Destroyed_MESH" :!label _label_2)
  (`PrimitiveComponent.SetCollisionProfileName` (`self.VentCover`) "NoCollision" true)
  (`PrimitiveComponent.SetCollisionProfileName` (`self.VisionBlocker`) "NoCollision" true)
  (set `self.StatusHealthState` "IsDead"))

(event `SetBroken`
  (goto _label_2))

(event `self.OnRepairDoor`
  (`parent.OnRepairDoor`)
  (`StaticMeshComponent.SetStaticMesh` (`self.VentCover`) "/Game/SurvivalGame/Dev/Meshes/DetatchableVentCover_Large_VentCover_MESH.DetatchableVentCover_Large_VentCover_MESH" :!label _label_3)
  (`PrimitiveComponent.SetCollisionProfileName` (`self.VentCover`) "BlockAllDynamic" true)
  (`PrimitiveComponent.SetCollisionProfileName` (`self.VisionBlocker`) "BlockAllDynamic" true)
  (set `self.StatusHealthState` "IsAlive"))

(event `SetRepaired`
  (goto _label_3))

(fn `UserConstructionScript`
  (`|ExecutionSequence`
    (:`then_0`
      (switch `EDoorState` (`self.CurrentDoorState`)
        (:`IsClosed`
          (`self.SetDoorPosition` false))
        (:`IsOpen`
          (`self.SetDoorPosition` true))))
    (:`then_1`
      (switch `EHealthState` (`self.StatusHealthState`)
        (:`IsAlive`
          (`self.SetRepaired`))
        (:`IsDead`
          (`self.SetBroken`))))))