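; Dev robot AI character that patrols a node path and visually tracks hostile targets with a camera mount.
; It claims and leaves path nodes to avoid conflicts, pausing between moves, and runs a behavior tree when possessed.
; Perception updates tint its lights by team attitude and set or clear the target enemy.
; Tick smoothly turns the camera, which also supplies eye rotation, toward targets within pitch/yaw bounds, otherwise toward body facing.
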(event `self.ReceiveTick`
  (params (DeltaSeconds :type "Float (single-precision)"))
  (if (`self.CanTrackTarget`)
    (`|ExecutionSequence`
      (:`then_0`
        (`/Engine/EditorBlueprintResources/StandardMacros.IsValid` (`self.TargetEnemy`)
          (:`Is Valid`
            (`self.SetTargetLookRotation` (`KismetMathLibrary.FindLookAtRotation` (`SceneComponent.K2_GetComponentLocation` (`self.CameraMount`)) (`self.K2_GetActorLocation` (`self.TargetEnemy`)))))))
      (:`then_1`
        (if (not (== (`self.CurrentLookRotation`) (`self.GetTargetLookRotation`) :`ErrorTolerance` 0.01))
          (bind _output_get (set `self.CurrentLookRotation` (`KismetMathLibrary.RInterpTo` (`self.CurrentLookRotation`) (`self.GetTargetLookRotation`) DeltaSeconds 5.0)))
          (`SceneComponent.K2_SetWorldRotation` (`self.CameraMount`) _output_get false false))))))

(event `self.ReceiveBeginPlay`
  (bind _returnvalue (`PatrolPath.GetNode` (`self.PatrolPathRef`) (`self.CurrentNodeID`)))
  (`PatrolNode.ClaimNode` _returnvalue self)
  (`|AIMoveTo` self (0.0 0.0 0.0) _returnvalue 10.0
    (:`OnSuccess`
      (`self.GotoNextNode`))))

(event `self.ReceivePossessed`
  (params (NewController :type "Controller Object Reference"))
  (bind _asteam_aicontroller (cast `TeamAIController` NewController))
  (`AIController.RunBehaviorTree` _asteam_aicontroller (`self.BehaviorTreeRef`)))

(event `GotoNextNode`
  (if (`PatrolNode.CanClaimNode` (`PatrolPath.GetNode` (`self.PatrolPathRef`) (`PatrolPath.GetNextNodeID` (`self.PatrolPathRef`) (`self.CurrentNodeID`) "Forward")) self)
    (bind _returnvalue (`PatrolNode.LeaveNode` (`PatrolPath.GetNode` (`self.PatrolPathRef`) (`self.CurrentNodeID`)) self))
    (if _returnvalue
      (set `self.CurrentNodeID` (`PatrolPath.GetNextNodeID` (`self.PatrolPathRef`) (`self.CurrentNodeID`) "Forward"))
      (bind _returnvalue_2 (`PatrolNode.ClaimNode` (`PatrolPath.GetNode` (`self.PatrolPathRef`) (`self.CurrentNodeID`)) self))
      (if _returnvalue_2
        (`|AIMoveTo` self (0.0 0.0 0.0) (`PatrolPath.GetNode` (`self.PatrolPathRef`) (`self.CurrentNodeID`)) 10.0
          (:`OnSuccess`
            (`self.K2_SetActorRotation` (`self.K2_GetActorRotation` (`PatrolPath.GetNode` (`self.PatrolPathRef`) (`self.CurrentNodeID`)))))
          (:`OnFail`
            _)))))
  (`KismetSystemLibrary.Delay` 5.0)
  (`self.GotoNextNode`))

(event `self.AIPerceptionComponentRef.OnTargetPerceptionInfoUpdated`
  (params (UpdateInfo :type "ActorPerceptionUpdateInfo Structure (by ref)"))
  (bind ((`Target` _target) (`Stimulus` _stimulus)) (break `ActorPerceptionUpdateInfo` UpdateInfo))
  (bind _returnvalue (`TeamAIController.GetTeamAttitudeTowards_BP` (`self.TeamAIControllerRef`) _target))
  (bind _returnvalue_2 (and (`KismetSystemLibrary.IsValid` _target) (`.bSuccessfullySensed` (break `AIStimulus` _stimulus))))
  (bind _returnvalue_3 (select `bool` _returnvalue_2 :`false` (struct :`R` 1.0 :`G` 1.0 :`B` 1.0 :`A` 1.0) :`true` (select `ETeamAttitude` _returnvalue :`Friendly` (struct :`G` 1.0 :`A` 1.0) :`Neutral` (struct :`G` 1.0 :`B` 1.0 :`A` 1.0) :`Hostile` (struct :`R` 1.0 :`A` 1.0) :!type "LinearColor Structure")))
  (`LightComponent.SetLightColor` (`self.PointLight`) _returnvalue_3 true)
  (`LightComponent.SetLightColor` (`self.SpotLight`) _returnvalue_3 true)
  (`/Engine/EditorBlueprintResources/StandardMacros.IsValid` (`self.TargetEnemy`)
    (:`Is Valid`
      (if (== _target (`self.TargetEnemy`))
        (if _returnvalue_2 :!label _label
          (if (`|EnumEquality` _returnvalue "Hostile")
            (`self.LookAtEnemy` _target))
          (else
            (`self.LookAtEnemy` null)))))
    (:`Is Not Valid`
      (goto _label))))

(event `LookAtEnemy`
  (params (Target :type "Actor Object Reference"))
  (if (!= Target (`self.TargetEnemy`))
    (bind _output_get (set `self.TargetEnemy` Target))
    (`/Engine/EditorBlueprintResources/StandardMacros.IsValid` _output_get
      (:`Is Valid`
        (`self.SetTargetLookRotation` (`KismetMathLibrary.FindLookAtRotation` (`SceneComponent.K2_GetComponentLocation` (`self.CameraMount`)) (`self.K2_GetActorLocation` (`self.TargetEnemy`)))))
      (:`Is Not Valid`
        (set `self.TargetLookRotation` (`self.K2_GetActorRotation`))))))

(fn `GetActorEyesLocation`
  (returns (ReturnValue :type "Vector Structure"))
  (return (`SceneComponent.K2_GetComponentLocation` (`self.CameraMesh`))))

(fn `GetActorEyesRotation`
  (returns (ReturnValue :type "Rotator Structure"))
  (return (`SceneComponent.K2_GetComponentRotation` (`self.CameraMount`))))

(fn `GetTargetLookRotation`
  (returns (Rotation :type "Rotator Structure"))
  (return (select `bool` (`KismetSystemLibrary.IsValid` (`self.TargetEnemy`)) :`false` (`self.K2_GetActorRotation`) :`true` (`self.TargetLookRotation`))))

(fn `SetTargetLookRotation`
  (params (NewRotation :type "Rotator Structure"))
  (bind (_x _y) (`KismetMathLibrary.BreakVector2D` (`self.RotationYawBounds`)))
  (bind (_x_2 _y_2) (`KismetMathLibrary.BreakVector2D` (`self.RotationPitchBounds`)))
  (bind _returnvalue (- (.pitch (`self.K2_GetActorRotation`)) (.pitch NewRotation)))
  (bind _returnvalue_2 (- (.yaw (`self.K2_GetActorRotation`)) (.yaw NewRotation)))
  (if (and (and (>= _returnvalue _x_2) (<= _returnvalue _y_2)) (and (>= _returnvalue_2 _x) (<= _returnvalue_2 _y)))
    (set `self.TargetLookRotation` NewRotation)
    (else
      (set `self.TargetLookRotation` (`self.K2_GetActorRotation`)))))

(fn `UserConstructionScript`)