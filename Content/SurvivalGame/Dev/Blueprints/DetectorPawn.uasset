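; DetectorPawn is an AI pawn that signals perceived targets with a point light colored by team attitude.
; On possession it drops old perception bindings, passes its TeamID to the TeamAIController and binds to that controller's AIPerception component.
; Target info updates show the light when sensing succeeds, tinted for friendly, neutral or hostile, and hide it otherwise.
; The other two perception handlers are empty stubs.
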(event `self.ReceivePossessed`
  (params (NewController :type "Controller Object Reference"))
  (`parent.ReceivePossessed` NewController)
  (`|ExecutionSequence`
    (:`then_0`
      (`/Engine/EditorBlueprintResources/StandardMacros.IsValid` (`self.PerceptionComponentRef`)
        (:`Is Valid`
          (remove `AIPerceptionComponent.OnPerceptionUpdated` (`self.PerceptionComponentRef`) (`|CreateDelegate` :!event `OnPerceptionUpdated`))
          (remove `AIPerceptionComponent.OnTargetPerceptionInfoUpdated` (`self.PerceptionComponentRef`) (`|CreateDelegate` :!event `OnTargetPerceptionInfoUpdated`))
          (remove `AIPerceptionComponent.OnTargetPerceptionUpdated` (`self.PerceptionComponentRef`) (`|CreateDelegate` :!event `OnTargetPerceptionUpdated`)))))
    (:`then_1`
      (bind _asteam_aicontroller (cast `TeamAIController` NewController))
      (bind _output_get (set `self.TeamControllerRef` _asteam_aicontroller))
      (`TeamAIController.SetTeamID` _output_get (`self.TeamID`))
      (set `self.PerceptionComponentRef` (`self.GetComponentByClass` (`self.TeamControllerRef`) "/Script/AIModule.AIPerceptionComponent"))
      (`/Engine/EditorBlueprintResources/StandardMacros.IsValid` (`self.PerceptionComponentRef`)
        (:`Is Valid`
          (add `AIPerceptionComponent.OnPerceptionUpdated` (`self.PerceptionComponentRef`) (`|CreateDelegate` :!event `OnPerceptionUpdated`))
          (add `AIPerceptionComponent.OnTargetPerceptionInfoUpdated` (`self.PerceptionComponentRef`) (`|CreateDelegate` :!event `OnTargetPerceptionInfoUpdated`))
          (add `AIPerceptionComponent.OnTargetPerceptionUpdated` (`self.PerceptionComponentRef`) (`|CreateDelegate` :!event `OnTargetPerceptionUpdated`)))))))

(event `SetLightVis`
  (params (IsVisible :type Boolean) (NewLightColor :type "LinearColor Structure"))
  (`SceneComponent.SetVisibility` (`self.PointLight`) IsVisible false)
  (`LightComponent.SetLightColor` (`self.PointLight`) NewLightColor true))

(fn `OnPerceptionUpdated`
  (params (UpdatedActors :type "Array of Actor Object Reference (by ref)"))
  (return))

(fn `OnTargetPerceptionInfoUpdated`
  (params (UpdateInfo :type "ActorPerceptionUpdateInfo Structure (by ref)"))
  (bind ((`Target` _target) (`Stimulus` _stimulus)) (break `ActorPerceptionUpdateInfo` UpdateInfo))
  (`|ExecutionSequence`
    (:`then_0`
      (`/Engine/EditorBlueprintResources/StandardMacros.IsValid` _target
        (:`Is Valid`
          (`self.SetLightVis` (`.bSuccessfullySensed` (break `AIStimulus` _stimulus)) (select `ETeamAttitude` (`TeamAIController.GetTeamAttitudeTowards_BP` (`self.TeamControllerRef`) _target) :`Friendly` (struct :`G` 1.0 :`A` 1.0) :`Neutral` (struct :`G` 1.0 :`B` 1.0 :`A` 1.0) :`Hostile` (struct :`R` 1.0 :`A` 1.0) :!type "LinearColor Structure")))
        (:`Is Not Valid`
          (`self.SetLightVis` false (struct :`R` 1.0 :`G` 1.0 :`B` 1.0 :`A` 1.0)))))
    (:`then_1`
      (return))))

(fn `OnTargetPerceptionUpdated`
  (params (Actor :type "Actor Object Reference") (Stimulus :type "AIStimulus Structure")))

(fn `UserConstructionScript`)