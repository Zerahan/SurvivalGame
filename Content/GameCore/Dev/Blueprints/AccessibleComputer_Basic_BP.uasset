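; Basic accessible computer that the player interacts with to use an operating system UI hosted on its Widget component.
; On BeginPlay it caches and initializes the ComputerOSWidget with itself, then prints a warning if app ID 0 is invalid.
; Beginning interaction switches the player controller to game-and-UI input with cursor and widget focus, while ending or cancelling restores game-only input.
; OpenApp simply defers to the parent class.
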(event `self.ReceiveBeginPlay`
  (bind _returnvalue (`WidgetComponent.GetWidget` (`self.Widget`)))
  (`parent.ReceiveBeginPlay`)
  (`/Engine/EditorBlueprintResources/StandardMacros.IsValid` _returnvalue
    (:`Is Valid`
      (bind _ascomputer_oswidget (cast `/Game/GameCore/Dev/UI/Computer/ComputerOSWidget` _returnvalue))
      (set `self.OperatingSystemWidget` _ascomputer_oswidget)
      (`/Game/GameCore/Dev/UI/Computer/ComputerOSWidget.Initialize` (`self.OperatingSystemWidget`) self)
      (`/Engine/EditorBlueprintResources/StandardMacros.IsValid` (`self.GetAppFromID` 0)
        (:`Is Not Valid`
          (`KismetSystemLibrary.PrintString` "Invalid"))))))

(event `InteractionInterface.BeginInteraction`
  (params (Info :type "InteractionInfo Structure"))
  (bind _operatingsystemwidget (`self.OperatingSystemWidget`))
  (`parent.BeginInteraction` Info)
  (bind _asplayer_controller (cast `PlayerController` (`.ControllerRef` (break `InteractionInfo` Info))))
  (`WidgetBlueprintLibrary.SetInputMode_GameAndUIEx` _asplayer_controller _operatingsystemwidget)
  (set `PlayerController.bShowMouseCursor` true _asplayer_controller)
  (`Widget.SetFocus` _operatingsystemwidget))

(event `InteractionInterface.EndInteraction`
  (params (Info :type "InteractionInfo Structure"))
  (`parent.EndInteraction` Info)
  (bind _asplayer_controller (cast `PlayerController` (`.ControllerRef` (break `InteractionInfo` Info))))
  (`WidgetBlueprintLibrary.SetInputMode_GameOnly` _asplayer_controller)
  (set `PlayerController.bShowMouseCursor` false _asplayer_controller))

(event `InteractionInterface.CancelInteraction`
  (params (Info :type "InteractionInfo Structure"))
  (`parent.CancelInteraction` Info)
  (bind _asplayer_controller (cast `PlayerController` (`.ControllerRef` (break `InteractionInfo` Info))))
  (`WidgetBlueprintLibrary.SetInputMode_GameOnly` _asplayer_controller)
  (set `PlayerController.bShowMouseCursor` false _asplayer_controller))

(fn `OpenApp`
  (params (TargetAppID :type Integer))
  (returns (ConsoleMessage :type String))
  (bind _consolemessage (`parent.OpenApp` TargetAppID))
  (return _consolemessage))

(fn `UserConstructionScript`
  (`parent.UserConstructionScript`))