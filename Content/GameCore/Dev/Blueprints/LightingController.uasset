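; LightingController switches lighting setups by streaming in a separate sublevel for each combination of active lights.
; Set and toggle events edit an array of light IDs, inserting in sorted order so each combination yields one canonical level name from prefix plus IDs.
; When that name changes, it loads the new level and unloads the previous one with blocking flags, ignoring light changes while IsLoadingLevel is set.
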(event `self.ReceiveBeginPlay`
  (bind _output_get (set `self.CurrentLevelName` (`KismetStringLibrary.Conv_StringToName` (`self.LightLevelPrefix`))))
  (set `self.LastLevelName` _output_get)
  (`GameplayStatics.LoadStreamLevel` (`self.CurrentLevelName`) true true))

(event `SetLightEnabled`
  (params (IsEnabled :type Boolean) (LightID :type String))
  (bind _returnvalue (`KismetArrayLibrary.Array_Find` (`self.ActiveLights`) LightID))
  (if (not (`self.IsLoadingLevel`))
    (if (and (== _returnvalue -1) IsEnabled)
      (`self.InsertNewLightID` LightID)
      (else
        (`KismetArrayLibrary.Array_Remove` (`self.ActiveLights`) _returnvalue)))
    (bind _success (`self.RebuildLevelName`))
    (if _success
      (`self.UpdateLighting`))))

(event `ToggleLight`
  (params (LightID :type String))
  (bind _returnvalue (`KismetArrayLibrary.Array_Find` (`self.ActiveLights`) LightID))
  (if (not (`self.IsLoadingLevel`))
    (if (!= _returnvalue -1)
      (`KismetArrayLibrary.Array_Remove` (`self.ActiveLights`) _returnvalue)
      (else
        (`self.InsertNewLightID` LightID)))
    (bind _success (`self.RebuildLevelName`))
    (if _success
      (`self.UpdateLighting`))))

(event `UpdateLighting`
  (if (not (`self.IsLoadingLevel`))
    (set `self.IsLoadingLevel` true)
    (`GameplayStatics.LoadStreamLevel` (`self.CurrentLevelName`) true true)
    (`GameplayStatics.UnloadStreamLevel` (`self.LastLevelName`) true)
    (set `self.IsLoadingLevel` false)))

(fn `CanChangeLight`
  (returns (ReturnValue :type Boolean))
  (return (not (`self.IsLoadingLevel`))))

(fn `InsertNewLightID`
  (params (LightID :type "String (by ref)"))
  (locals (LocalInsertIndex :type Integer))
  (for _index (range (`KismetArrayLibrary.Array_Length` (`self.ActiveLights`)))
    (bind _returnvalue (`UtilityFunctionLibrary.CompareString` (`|GetArrayItem` (`self.ActiveLights`) _index) (`local.LightID`)))
    (if (!= _returnvalue -1)
      (`KismetArrayLibrary.Array_Insert` (`self.ActiveLights`) (`local.LightID`) _index)
      (return)))
  (`KismetArrayLibrary.Array_Add` (`self.ActiveLights`) (`local.LightID`))
  (return))

(fn `RebuildLevelName`
  (returns (Success :type Boolean))
  (locals (LocalNewLightString :type String))
  (for _array_element (`self.ActiveLights`)
    (set `local.LocalNewLightString` (`KismetStringLibrary.Concat_StrStr` (`local.LocalNewLightString`) _array_element)))
  (if (`KismetStringLibrary.NotEqual_StrStr` (`KismetStringLibrary.Conv_NameToString` (`self.CurrentLevelName`)) (`KismetStringLibrary.Concat_StrStr` (`self.LightLevelPrefix`) (`local.LocalNewLightString`)))
    (set `self.LastLevelName` (`self.CurrentLevelName`))
    (set `self.CurrentLevelName` (`KismetStringLibrary.Conv_StringToName` (`KismetStringLibrary.Concat_StrStr` (`self.LightLevelPrefix`) (`local.LocalNewLightString`))))
    (return true)
    (else
      (return false))))

(fn `UserConstructionScript`)